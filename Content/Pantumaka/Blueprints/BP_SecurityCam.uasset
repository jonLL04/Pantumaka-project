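; BP_SecurityCam is a security camera that can sweep side to side and serve as the player's view.
; On BeginPlay, if CanRotate is set, it waits a short random delay, staggering multiple cameras, then plays the RotateCamera timeline.
; The timeline's Alpha drives a yaw lerp on the Holder component's relative rotation.
; SwitchToCamera makes this actor the view target of the first player controller.
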(event Custom|SwitchToCamera
  (Game|Player|SetViewTargetwithBlend (Game|GetPlayerController 0) self 0.0 "VTBlend_Linear" 0.0 false))

(event EventBeginPlay
  (if (Variables|Default|GetCanRotate)
    ;[1 1 1] Add Ramdom
    (Utilities|FlowControl|Delay (Math|Random|RandomFloatinRange 0.0 5.0))
    (Audio|Components|Audio|Play (Variables|Default|GetRotateCamera))))

(fn ConstructionScript)